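; Grid actor that divides a world-sized area into tiles and visualizes them with debug drawing, in construction and at BeginPlay.
; DrawTile steps from a computed corner, sphere-tracing two channels per tile and drawing green or brown planes on hits.
; GenerateMapDataFromWorld stores ground type, location and index in TilesData, reading BP_Obstacle on second-channel hits.
; That function looks unfinished: it first traces world origin, and its tile loop only draws.
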(event `self.ReceiveBeginPlay`
  (`self.GetBottomLeft`)
  (`self.DrawTile`))

(fn `DrawTile`
  (bind _returnvalue (- (`self.TileSize`) 5.0))
  (bind (_horizontaltiles _verticaltiles) (`self.GetTileNumber`))
  (for _index (range (+ (`KismetMathLibrary.FTrunc` _verticaltiles) 1))
    (for _index_2 (range (+ (`KismetMathLibrary.FTrunc` _horizontaltiles) 1))
      (bind _bottomleft (`self.GetBottomLeft`))
      (bind _output_get (set `self.TileLocation` (+ _bottomleft (* (`SceneComponent.GetRightVector` (`self.Scene`)) (* _index (* -2.0 (`self.TileSize`)))) (* (`SceneComponent.GetForwardVector` (`self.Scene`)) (* _index_2 (* 2.0 (`self.TileSize`)))))))
      (`|ExecutionSequence`
        (:`then_0`
          (bind _returnvalue_2 (+ _output_get (0.01 0.0 0.0)))
          (bind (_outhit _returnvalue_3) (`KismetSystemLibrary.SphereTraceSingle` :`Start` _output_get :`End` _returnvalue_2 :`Radius` 5.0 :`TraceChannel` "TraceTypeQuery3" :`DrawDebugType` "Persistent" :`DrawTime` 10000000.0))
          (if _returnvalue_3
            (bind _z (.z _output_get))
            (`KismetSystemLibrary.DrawDebugPlane` (make `Plane` _z 0.0 0.0 1.0) _output_get _returnvalue (struct :`R` 0.145264 :`G` 0.796875 :`B` 0.2624 :`A` 1.0) 100000.0)))
        (:`then_1`
          (bind (_outhit_2 _returnvalue_4) (`KismetSystemLibrary.SphereTraceSingle` :`Start` _output_get :`End` _returnvalue_2 :`Radius` 5.0 :`TraceChannel` "TraceTypeQuery4" :`DrawDebugType` "Persistent" :`DrawTime` 10000000.0))
          (if _returnvalue_4
            (`KismetSystemLibrary.DrawDebugPlane` (make `Plane` _z 0.0 0.0 1.0) _output_get _returnvalue (struct :`R` 0.3125 :`G` 0.184663 :`B` 0.078103 :`A` 1.0) 100000.0)))))))

(fn `GenerateMapDataFromWorld`
  (bind _returnvalue (- (`self.TileSize`) 5.0))
  (bind _returnvalue_2 (`KismetMathLibrary.MakeVector2D` (`KismetMathLibrary.Conv_IntToDouble` (`self.X`)) (`KismetMathLibrary.Conv_IntToDouble` (`self.Y`))))
  (bind _returnvalue_3 (`KismetMathLibrary.MakeVector2D` (`KismetMathLibrary.Conv_IntToDouble` (`self.X`)) (`KismetMathLibrary.Conv_IntToDouble` (`self.Y`))))
  (bind _returnvalue_4 (`KismetMathLibrary.MakeVector2D` (`KismetMathLibrary.Conv_IntToDouble` (`self.X`)) (`KismetMathLibrary.Conv_IntToDouble` (`self.Y`))))
  (bind _incollision (`self.Tile Sphere Trace` (0.0 0.0 0.0) "TraceTypeQuery3"))
  (if _incollision
    (bind (_incollision_2 _collided_actor) (`self.Tile Sphere Trace` (`self.TileLocation`) "TraceTypeQuery4"))
    (if _incollision_2
      (bind _asbp_obstacle (cast `/Game/Blueprints/BP_Obstacle` _collided_actor))
      (`BlueprintMapLibrary.Map_Add` (`self.TilesData`) _returnvalue_3 (make `/Game/Blueprints/Struct_Tile` (`/Game/Blueprints/BP_Obstacle.GroundType` _asbp_obstacle) (`self.TileLocation`) _returnvalue_3))
      (else
        (`BlueprintMapLibrary.Map_Add` (`self.TilesData`) _returnvalue_4 (make `/Game/Blueprints/Struct_Tile` "NewEnumerator1" (`self.TileLocation`) _returnvalue_4))
        (bind (_horizontaltiles _verticaltiles) (`self.GetTileNumber`))
        (for _index (range (+ (`KismetMathLibrary.FTrunc` _verticaltiles) 1))
          (for _index_2 (range (+ (`KismetMathLibrary.FTrunc` _horizontaltiles) 1))
            (bind _bottomleft (`self.GetBottomLeft`))
            (bind _output_get (set `self.TileLocation` (+ _bottomleft (* (`SceneComponent.GetRightVector` (`self.Scene`)) (* _index (* -2.0 (`self.TileSize`)))) (* (`SceneComponent.GetForwardVector` (`self.Scene`)) (* _index_2 (* 2.0 (`self.TileSize`)))))))
            (`|ExecutionSequence`
              (:`then_0`
                (bind _returnvalue_5 (+ _output_get (0.01 0.0 0.0)))
                (bind (_outhit _returnvalue_6) (`KismetSystemLibrary.SphereTraceSingle` :`Start` _output_get :`End` _returnvalue_5 :`Radius` 5.0 :`TraceChannel` "TraceTypeQuery3" :`DrawDebugType` "Persistent" :`DrawTime` 10000000.0))
                (if _returnvalue_6
                  (bind _z (.z _output_get))
                  (`KismetSystemLibrary.DrawDebugPlane` (make `Plane` _z 0.0 0.0 1.0) _output_get _returnvalue (struct :`R` 0.145264 :`G` 0.796875 :`B` 0.2624 :`A` 1.0) 100000.0)))
              (:`then_1`
                (bind (_outhit_2 _returnvalue_7) (`KismetSystemLibrary.SphereTraceSingle` :`Start` _output_get :`End` _returnvalue_5 :`Radius` 5.0 :`TraceChannel` "TraceTypeQuery4" :`DrawDebugType` "Persistent" :`DrawTime` 10000000.0))
                (if _returnvalue_7
                  (`KismetSystemLibrary.DrawDebugPlane` (make `Plane` _z 0.0 0.0 1.0) _output_get _returnvalue (struct :`R` 0.3125 :`G` 0.184663 :`B` 0.078103 :`A` 1.0) 100000.0))))))))
    (else
      (`BlueprintMapLibrary.Map_Add` (`self.TilesData`) _returnvalue_2 (make `/Game/Blueprints/Struct_Tile` "NewEnumerator0" (`self.TileLocation`) _returnvalue_2)))))

(fn `GetBottomLeft`
  (returns (BottomLeft :type "Vector Structure"))
  (locals (NewLocalVar :type "Vector Structure" :default (0.0 0.0 0.0)))
  (bind (_gridsizeworld_x _gridsizeworld_y) (`KismetMathLibrary.BreakVector2D` (`self.GridSizeWorld`)))
  (bind _returnvalue (- (* (`SceneComponent.GetRightVector` (`self.Scene`)) _gridsizeworld_x) (* _gridsizeworld_y (`SceneComponent.GetForwardVector` (`self.Scene`)))))
  (`KismetSystemLibrary.DrawDebugBox` _returnvalue (10.0 10.0 0.1) (struct :`G` 0.703602 :`B` 1.0 :`A` 1.0) (struct) 100000000.0 10.0)
  (return _returnvalue))

(fn `GetTileNumber`
  (returns (HorizontalTiles :type "Float (double-precision)") (VerticalTiles :type "Float (double-precision)"))
  (bind (_returnvalue_x _returnvalue_y) (`KismetMathLibrary.BreakVector2D` (/ (`self.GridSizeWorld`) (`self.TileSize`))))
  (return _returnvalue_x _returnvalue_y))

(fn `Tile Sphere Trace`
  (params (Location :type "Vector Structure") (`Trace Channel` :type "ETraceTypeQuery Enum" :default "TraceTypeQuery1"))
  (returns (InCollision :type Boolean) (`Collided Actor` :type "Object Object Reference"))
  (bind (_outhit _returnvalue) (`KismetSystemLibrary.SphereTraceSingle` :`Start` Location :`End` (+ Location (0.1 0.0 0.0)) :`Radius` 10.0 :`TraceChannel` `Trace Channel` :`DrawDebugType` "Persistent" :`DrawTime` 100000.0))
  (return _returnvalue (`.HitActor` (`GameplayStatics.BreakHitResult` _outhit))))

(fn `UserConstructionScript`
  (bind (_gridsizeworld_x _gridsizeworld_y) (`KismetMathLibrary.BreakVector2D` (`self.GridSizeWorld`)))
  (`KismetSystemLibrary.FlushPersistentDebugLines`)
  (set `self.GridLocation` (`SceneComponent.K2_GetComponentLocation` (`self.Scene`)))
  (`KismetSystemLibrary.DrawDebugBox` (`self.GridLocation`) (`KismetMathLibrary.MakeVector` _gridsizeworld_x _gridsizeworld_y) (`self.GridColor`) (struct) 10000.0 10.0)
  (`self.GenerateMapDataFromWorld`)
  (`self.DrawTile`))